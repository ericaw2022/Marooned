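; DialogueComponent_BP runs a dialogue through a behavior tree when the player interacts with it.
; It spawns a dedicated DialogueAIController at BeginPlay to host DialogueTree.
; On interaction it shows a Narrative2 widget with UI-only input and cursor, starts the tree, and passes the widget through DialogueBlackboard.
; The widget's exit event stops the tree logic, removes the widget and restores game input.
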(event Custom|OnExit
  (bind _narrative2 (Variables|Default|GetNarrative2))
  (bind _returnvalue (Widget|GetOwningPlayer _narrative2))
  (Input|SetInputModeGameOnly _returnvalue false)
  (Variables|/Script/Engine.PlayerController|SetbShowMouseCursor _returnvalue false)
  (AI|Logic|StopLogic (Variables|/Script/AIModule.AIController|GetBrainComponent (Variables|Default|GetAIController)) "Dialogue Exit")
  (Widget|RemovefromParent (Variables|Default|GetNarrative2)))

(event EventBeginPlay
  (bind _returnvalue (Game|SpawnActorfromClass "/Game/Jenkins_Amaris/BluePrints/DialogueAIController.DialogueAIController_C" (Math|Transform|MakeTransform "0, 0, 0" "0, 0, 0" "1.000000,1.000000,1.000000") "Undefined" "MultiplyWithRoot" 0 0))
  (Variables|Default|SetAIController _returnvalue))

(event EventTick
  (params (DeltaSeconds :type Float%20%28single-precision%29)))

(event EventOnInteraction
  (params (PlayerCharacter :type Williams%20Player%20BP%20Object%20Reference))
  (bind _returnvalue (Pawn|GetController PlayerCharacter))
  (bind _asplayer_controller (Utilities|Casting|CastToPlayerController _returnvalue))
  (bind _returnvalue_2 (UserInterface|CreateWidget "/Game/Jenkins_Amaris/Widgets/Narrative2.Narrative2_C" _asplayer_controller))
  (bind _output_get (Variables|Default|SetNarrative2 _returnvalue_2))
  (EventDispatchers|BindEventtoOnExit _output_get (delegate Custom|OnExit))
  (UserInterface|Viewport|AddtoViewport _output_get 0)
  (Input|SetInputModeUIOnly _asplayer_controller _output_get "DoNotLock" false)
  (Variables|/Script/Engine.PlayerController|SetbShowMouseCursor _asplayer_controller true)
  (AI|RunBehaviorTree (Variables|Default|GetAIController) (Variables|Default|GetDialogueTree))
  (bind _blackboardcomponent (Class|AIController|UseBlackboard (Variables|Default|GetAIController) "/Game/Jenkins_Amaris/BluePrints/DialogueBlackboard.DialogueBlackboard"))
  (AI|Components|Blackboard|SetValueasObject _blackboardcomponent (Utilities|Name|MakeLiteralName "Narrative2") (Variables|Default|GetNarrative2)))
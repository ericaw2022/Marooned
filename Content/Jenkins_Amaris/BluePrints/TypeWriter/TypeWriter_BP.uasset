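; TypeWriter_BP is a Blueprint that sends dialogue text to the player character for display, with a configurable text delay.
; Its Speaking event first checks the character's CheckTalkingMessage and, when that returns false, calls TalkingMessage with the Text and TextDelay variables.
; It then advances CurrentDialogue and wraps it to zero at the end of the Dialogue array, though the indexed array entry is left unconnected.
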(event Custom|Speaking
  (bind _returnvalue (Game|GetPlayerCharacter 0))
  (bind _btaking (Class|TypewritingSystem|CheckTalking(Message) _returnvalue))
  (if (not _btaking)
    (Class|TypewritingSystem|Talking(Message) _returnvalue (Variables|Default|GetText) (Variables|Default|GetTextDelay))
    (bind _result (Math|Integer|IncrementInt (Variables|Default|GetCurrentDialogue))
      (:%20%20
        (if (>= _result (Utilities|Array|Length (Variables|Default|GetDialogue)))
          (Variables|Default|SetCurrentDialogue 0))))))
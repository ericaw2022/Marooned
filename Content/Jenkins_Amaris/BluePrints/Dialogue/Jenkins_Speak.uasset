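; Behavior tree task for dialogue that has an actor or object of type Narrative2 speak a line of text.
; On execute, it reads the Narrative2 object from the blackboard, binds to its OnSpeakFinished dispatcher and calls Speak with the Text variable.
; When speech finishes, it unbinds the event and finishes successfully, so the tree waits for each line to end.
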(event Custom|OnSpeakFinished
  (EventDispatchers|UnbindEventfromOnSpeakFinished (.AsNarrative%202 (Utilities|Casting|CastToNarrative2 (Class|BTFunctionLibrary|GetBlackboardValueasObject (Variables|Default|GetNarrative2)))) (delegate Custom|OnSpeakFinished))
  (AI|BehaviorTree|FinishExecute true))

(event EventReceiveExecuteAI
  (params (OwnerController :type AI%20Controller%20Object%20Reference) (ControlledPawn :type Pawn%20Object%20Reference))
  (bind _narrative2 (Variables|Default|GetNarrative2))
  (bind _returnvalue (Class|BTFunctionLibrary|GetBlackboardValueasObject _narrative2))
  (bind _asnarrative_2 (Utilities|Casting|CastToNarrative2 _returnvalue))
  (EventDispatchers|AssignOnSpeakFinished _asnarrative_2 (EventDispatchers|CreateEvent :!event Custom|OnSpeakFinished))
  (Default|Speak _asnarrative_2 (Variables|Default|GetText)))
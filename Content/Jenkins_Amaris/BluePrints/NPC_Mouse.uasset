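; NPC_Mouse is a mouse NPC that brings up narrative options when the player presses Interact nearby.
; If PlayerNearby is set, the input disables player character input, adds a Narrative_Options widget to the viewport and shows the mouse cursor.
; The Interact event is empty, and an unconnected DialogueMouse conversation call never runs.
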(event EventInteract
  (params (Instigator :type Actor%20Object%20Reference)))

(event Input|ActionEvents|InputActionInteract
  (params (Key :type Key%20Structure :default "None"))
  (bind _returnvalue (Game|GetPlayerController 0))
  (:Pressed
    (if (Variables|Default|GetPlayerNearby)
      (Input|DisableInput (Game|GetPlayerCharacter 0) _returnvalue)
      (bind _returnvalue_2 (UserInterface|CreateWidget "/Game/Jenkins_Amaris/Widgets/Narrative_Options.Narrative_Options_C" 0 "" 0))
      (UserInterface|Viewport|AddtoViewport _returnvalue_2 0)
      (Variables|/Script/Engine.PlayerController|SetbShowMouseCursor _returnvalue true))))

(event Input|KeyboardEvents|E
  (params (Key :type Key%20Structure :default "None")))

(fn ConstructionScript
  (|CallParentFunction))
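; Behavior tree task that walks an AI pawn along the patrol path defined on its AiMovement component.
; The path is a map of point actors to wait times; on each arrival it notifies the point and starts a wait timer before stepping to the next index.
; At either end it loops to the start, reverses direction or finishes, per PatrolPathOutcome.
; It fails if the component or path is missing or a move fails.
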(event Custom|MoveToPatrolPoint
  (bind _patrol_path (Variables|AIMovement|GetPatrol%20Path))
  ;[1 1 1] Moving to patrol points
  (bind _keys (Utilities|Map|Keys (Variables|AIMovement|GetPatrol%20Path)))
  (AI|AIMoveTo (Variables|AIMovement|GetControlled%20Pawn) (Transformation|GetActorLocation (Utilities|Array|Get(acopy) _keys (Variables|AIMovement|GetCurrentPatrolIndex))) 0 5.0 false
    (:OnSuccess
      (bind _keys_2 (Utilities|Map|Keys _patrol_path))
      (Utilities|Time|SetTimerbyEvent (delegate Custom|OnEndWait) (Math|Float|Max(Float) (.Value (Utilities|Map|Find _patrol_path (Utilities|Array|Get(acopy) _keys_2 (Variables|AIMovement|GetCurrentPatrolIndex)))) 0.1))
      (Default|OnPatrollerEntered (Utilities|Array|Get(acopy) _keys_2 (Variables|AIMovement|GetCurrentPatrolIndex)) (.AsCharacter (Utilities|Casting|CastToCharacter (Variables|AIMovement|GetControlled%20Pawn)))))
    (:OnFail
      (AI|BehaviorTree|FinishExecute false))))

(event Custom|OnEndWait
  ;[1 1 1] Moving to patrol points
  (bind _output_get (Variables|AIMovement|SetCurrentPatrolIndex (+ (Variables|AIMovement|GetCurrentPatrolIndex) (Variables|AIMovement|GetPathDirection))))
  (if (CallFunction|IsValidMapIndex _output_get)
    (CallFunction|MovetoPatrolPoint)
    (else
      (switch Utilities|FlowControl|Switch|SwitchonJenkins_EPatrolPathOutCome (Variables|AIMovement|GetPatrol%20Path%20Outcome)
        (:NewEnumerator0
          (Variables|AIMovement|SetCurrentPatrolIndex 0)
          (CallFunction|MovetoPatrolPoint))
        (:NewEnumerator1
          (Variables|AIMovement|SetPathDirection (* (Variables|AIMovement|GetPathDirection) -1))
          (Variables|AIMovement|SetCurrentPatrolIndex (+ (Variables|AIMovement|GetCurrentPatrolIndex) (Variables|AIMovement|GetPathDirection)))
          (CallFunction|MovetoPatrolPoint))
        (:NewEnumerator2
          (AI|BehaviorTree|FinishExecute true))))))

(event EventReceiveExecuteAI
  (params (OwnerController :type AI%20Controller%20Object%20Reference) (ControlledPawn :type Pawn%20Object%20Reference))
  (bind _returnvalue (Actor|GetComponentbyClass ControlledPawn "/Game/Jenkins_Amaris/BluePrints/MovingNPC/AiMovement.AiMovement_C"))
  (bind _patrolpath (Variables|/Game/Jenkins_Amaris/BluePrints/MovingNPC/AiMovement.AiMovement_C|GetPatrolPath _returnvalue))
  ;[1 1 1] Getting simple component
  (Variables|AIMovement|SetControlled%20Pawn ControlledPawn)
  (Utilities|IsValid _returnvalue
    (:Is%20Valid
      (Variables|AIMovement|SetPatrol%20Path%20Outcome (Variables|/Game/Jenkins_Amaris/BluePrints/MovingNPC/AiMovement.AiMovement_C|GetPatrolPathOutcome _returnvalue))
      (if (> (Utilities|Map|Length _patrolpath) 0)
        (Variables|AIMovement|SetPatrol%20Path _patrolpath)
        (CallFunction|MovetoPatrolPoint)
        (else
          (AI|BehaviorTree|FinishExecute false))))
    (:Is%20Not%20Valid
      (AI|BehaviorTree|FinishExecute false))))

(fn IsValidMapIndex
  (params (IndexToTest :type Integer))
  (bind _keys (Utilities|Map|Keys (Variables|AIMovement|GetPatrol%20Path)))
  (return (Utilities|Array|IsValidIndex _keys IndexToTest)))
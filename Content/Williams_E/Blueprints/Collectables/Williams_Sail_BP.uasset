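; Collectable sail pickup that the player takes into their inventory through an Interact event.
; Interact increments the player's Sail count, then tries Comp_Inventory; the count rises even when the inventory is full.
; On success it plays a sound, refreshes the W_Inventory grid and destroys itself, otherwise it prints a full message.
; A sphere overlap toggles custom depth on the item mesh while the player is near.
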(event OnComponentBeginOverlap(Sphere)
  (params (OverlappedComponent :type Primitive%20Component%20Object%20Reference) (OtherActor :type Actor%20Object%20Reference) (OtherComp :type Primitive%20Component%20Object%20Reference) (OtherBodyIndex :type Integer) (bFromSweep :type Boolean) (SweepResult :type Hit%20Result%20Structure%20%28by%20ref%29))
  (if (== OtherActor (Game|GetPlayerCharacter 0))
    (Rendering|SetRenderCustomDepth (Variables|Default|GetItem) true)))

(event OnComponentEndOverlap(Sphere)
  (params (OverlappedComponent :type Primitive%20Component%20Object%20Reference) (OtherActor :type Actor%20Object%20Reference) (OtherComp :type Primitive%20Component%20Object%20Reference) (OtherBodyIndex :type Integer))
  (if (== OtherActor (Game|GetPlayerCharacter 0))
    (Rendering|SetRenderCustomDepth (Variables|Default|GetItem) false)))

(event EventBeginPlay)

(event Collision|EventActorBeginOverlap
  (params (OtherActor :type Actor%20Object%20Reference)))

(event EventTick
  (params (DeltaSeconds :type Float%20%28single-precision%29)))

(event EventInteract
  (bind _aswilliams_player_bp (Utilities|Casting|CastToWilliams_Player_BP (Game|GetPlayerCharacter 0)))
  (Variables|/Game/Williams_E/Blueprints/Player/Williams_Player_BP.Williams_Player_BP_C|SetSail _aswilliams_player_bp (+ (Variables|/Game/Williams_E/Blueprints/Player/Williams_Player_BP.Williams_Player_BP_C|GetSail _aswilliams_player_bp) 1))
  (bind _itemadded (Default|AddtoInventory (Actor|GetComponentbyClass _aswilliams_player_bp "/Game/Sean_H/Inventory/Comp_Inventory.Comp_Inventory_C") (Variables|Default|GetInventory_0)))
  (if _itemadded
    (bind _foundwidgets (Widget|GetAllWidgetsOfClass "/Game/Sean_H/Inventory/W_Inventory.W_Inventory_C" true))
    ;[0.1596 0.6662 1] Pickup Sound (Luis)
    (Audio|PlaySound2D "/Game/Robles_Delgado_L/Sounds/Player-Sounds/Item/Robles_Item_Pickup.Robles_Item_Pickup" 1.0 1.0 0.0 0 0)
    (Utilities|IsValid (Utilities|Array|Get(acopy) _foundwidgets)
      (:Is%20Valid
        (Default|SetGrid (Utilities|Array|Get(acopy) _foundwidgets)))
      (:Is%20Not%20Valid
        _))
    (Actor|DestroyActor)
    (Development|PrintString "Sail collected!")
    (else
      (Development|PrintString "Inventory Full"))))

(fn ConstructionScript)

(fn PickUpItem)
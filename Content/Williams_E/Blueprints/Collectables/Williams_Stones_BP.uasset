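; Collectable stone that the player picks up into their inventory, highlighted through custom depth while the player is inside its sphere.
; PickUp increments the player's Stones count, then tries adding the item to Comp_Inventory; the count rises even if that fails.
; On success it plays a sound, refreshes the W_Inventory grid, disables collision and uses a Timeline to pull the mesh toward the player before destroying itself.
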(event OnComponentBeginOverlap(Sphere)
  (params (OverlappedComponent :type Primitive%20Component%20Object%20Reference) (OtherActor :type Actor%20Object%20Reference) (OtherComp :type Primitive%20Component%20Object%20Reference) (OtherBodyIndex :type Integer) (bFromSweep :type Boolean) (SweepResult :type Hit%20Result%20Structure%20%28by%20ref%29))
  (if (== OtherActor (Game|GetPlayerCharacter 0))
    (Rendering|SetRenderCustomDepth (Variables|Default|GetItem) true)))

(event OnComponentEndOverlap(Sphere)
  (params (OverlappedComponent :type Primitive%20Component%20Object%20Reference) (OtherActor :type Actor%20Object%20Reference) (OtherComp :type Primitive%20Component%20Object%20Reference) (OtherBodyIndex :type Integer))
  (if (== OtherActor (Game|GetPlayerCharacter 0))
    (Rendering|SetRenderCustomDepth (Variables|Default|GetItem) false)))

(event EventBeginPlay)

(event Collision|EventActorBeginOverlap
  (params (OtherActor :type Actor%20Object%20Reference)))

(event EventTick
  (params (DeltaSeconds :type Float%20%28single-precision%29)))

(event EventPickUp
  (bind _player (Variables|Default|GetPlayer))
  (bind _item (Variables|Default|GetItem))
  (bind _returnvalue (Transformation|GetWorldLocation _item))
  (bind _rootcomponent (Variables|/Script/Engine.Actor|GetRootComponent _player))
  (bind _returnvalue_2 (Transformation|GetWorldLocation _rootcomponent))
  (bind _aswilliams_player_bp (Utilities|Casting|CastToWilliams_Player_BP (Game|GetPlayerCharacter 0)))
  (Variables|/Game/Williams_E/Blueprints/Player/Williams_Player_BP.Williams_Player_BP_C|SetStones _aswilliams_player_bp (+ (Variables|/Game/Williams_E/Blueprints/Player/Williams_Player_BP.Williams_Player_BP_C|GetStones _aswilliams_player_bp) 1))
  (bind _itemadded (Default|AddtoInventory (Actor|GetComponentbyClass _aswilliams_player_bp "/Game/Sean_H/Inventory/Comp_Inventory.Comp_Inventory_C") (Variables|Default|GetInventory_0)))
  (if _itemadded
    (bind _foundwidgets (Widget|GetAllWidgetsOfClass "/Game/Sean_H/Inventory/W_Inventory.W_Inventory_C" true))
    ;[0.1596 0.6662 1] Pickup Sound (Luis)
    (Audio|PlaySound2D "/Game/Robles_Delgado_L/Sounds/Player-Sounds/Item/Robles_Item_Pickup.Robles_Item_Pickup" 1.0 1.0 0.0 0 0)
    (Utilities|IsValid (Utilities|Array|Get(acopy) _foundwidgets)
      (:Is%20Valid
        (Default|SetGrid (Utilities|Array|Get(acopy) _foundwidgets)))
      (:Is%20Not%20Valid
        _))
    (Collision|SetCollisionEnabled (Variables|Default|GetItem) "NoCollision")
    (bind _pickup (Timeline|Timeline Play)
      (:Update
        (Transformation|SetWorldLocation _item (Math|Vector|MakeVector (Math|Float|Lerp (.x _returnvalue) (.x _returnvalue_2) _pickup) (Math|Float|Lerp (.y _returnvalue) (.y _returnvalue_2) _pickup) (Math|Float|Lerp (.z _returnvalue) (- (.z _returnvalue_2) 3e+01) _pickup)) false false))
      (:Finished
        (Actor|DestroyActor)))))

(fn ConstructionScript)
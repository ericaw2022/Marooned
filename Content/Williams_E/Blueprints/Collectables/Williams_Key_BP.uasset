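; Collectable cave key actor that the player picks up by interacting with it.
; Interact sets HasCaveKey on the player, then tries to add the item to the player's inventory component.
; On success it refreshes any open inventory widget's grid and destroys itself, printing a message.
; A full inventory prints a notice and leaves the key in place, though the flag is already set.
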(event EventInteract
  (bind _aswilliams_player_bp (Utilities|Casting|CastToWilliams_Player_BP (Game|GetPlayerCharacter 0)))
  (Variables|/Game/Williams_E/Blueprints/Player/Williams_Player_BP.Williams_Player_BP_C|SetHasCaveKey? _aswilliams_player_bp true)
  (bind _itemadded (Default|AddtoInventory (Actor|GetComponentbyClass _aswilliams_player_bp "/Game/Sean_H/Inventory/Comp_Inventory.Comp_Inventory_C") (Variables|Default|GetInventory)))
  (if _itemadded
    (bind _foundwidgets (Widget|GetAllWidgetsOfClass "/Game/Sean_H/Inventory/W_Inventory.W_Inventory_C" true))
    (Utilities|IsValid (Utilities|Array|Get(acopy) _foundwidgets)
      (:Is%20Valid
        (Default|SetGrid (Utilities|Array|Get(acopy) _foundwidgets)))
      (:Is%20Not%20Valid
        _))
    (Actor|DestroyActor)
    (Development|PrintString "key collected!")
    (else
      (Development|PrintString "Inventory Full"))))

(fn ConstructionScript)
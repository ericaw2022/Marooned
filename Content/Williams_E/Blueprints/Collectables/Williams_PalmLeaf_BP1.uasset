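; A collectable palm leaf actor that the player picks up by interacting with it.
; On Interact it adds its item data to the player's inventory component.
; On success it refreshes the open inventory widget's grid and destroys itself, printing a confirmation.
; If the inventory is full it only prints a message, and the PickUpItem function is empty.
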(event EventBeginPlay)

(event Collision|EventActorBeginOverlap
  (params (OtherActor :type Actor%20Object%20Reference)))

(event EventTick
  (params (DeltaSeconds :type Float%20%28single-precision%29)))

(event EventInteract
  (bind _aswilliams_player_bp (Utilities|Casting|CastToWilliams_Player_BP (Game|GetPlayerCharacter 0)))
  (bind _itemadded (Default|AddtoInventory (Actor|GetComponentbyClass _aswilliams_player_bp "/Game/Sean_H/Inventory/Comp_Inventory.Comp_Inventory_C") (Variables|Default|GetInventory)))
  (if _itemadded
    (bind _foundwidgets (Widget|GetAllWidgetsOfClass "/Game/Sean_H/Inventory/W_Inventory.W_Inventory_C" true))
    (Utilities|IsValid (Utilities|Array|Get(acopy) _foundwidgets)
      (:Is%20Valid
        (Default|SetGrid (Utilities|Array|Get(acopy) _foundwidgets)))
      (:Is%20Not%20Valid
        _))
    (Actor|DestroyActor)
    (Development|PrintString "Leaf collected!")
    (else
      (Development|PrintString "Inventory Full"))))

(fn ConstructionScript)

(fn PickUpItem)
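; Collectable fruit that the player can pick up into inventory or eat to get a hunger amount.
; On BeginPlay it picks a random mesh and fills its pickup widget; sphere overlap toggles custom depth for the player.
; PickUp increments player Food, then, if the inventory add succeeds, refreshes the grid and lerps the item to the player before destroying it.
; Eat plays a sound, calls DestroyFood and returns HungerAmount.
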(event OnComponentBeginOverlap(Sphere)
  (params (OverlappedComponent :type Primitive%20Component%20Object%20Reference) (OtherActor :type Actor%20Object%20Reference) (OtherComp :type Primitive%20Component%20Object%20Reference) (OtherBodyIndex :type Integer) (bFromSweep :type Boolean) (SweepResult :type Hit%20Result%20Structure%20%28by%20ref%29))
  (if (== OtherActor (Game|GetPlayerCharacter 0))
    (Rendering|SetRenderCustomDepth (Variables|Default|GetItem) true)))

(event OnComponentEndOverlap(Sphere)
  (params (OverlappedComponent :type Primitive%20Component%20Object%20Reference) (OtherActor :type Actor%20Object%20Reference) (OtherComp :type Primitive%20Component%20Object%20Reference) (OtherBodyIndex :type Integer))
  (if (== OtherActor (Game|GetPlayerCharacter 0))
    (Rendering|SetRenderCustomDepth (Variables|Default|GetItem) false)))

(event Custom|Set%20Random%20Mesh
  (bind _available_meshes (Variables|Default|GetAvailable%20Meshes))
  ;[1 1 1] Random Mesh
  (Components|StaticMesh|SetStaticMesh (Variables|Default|GetItem) (Utilities|Array|Get(acopy) _available_meshes (Math|Random|RandomIntegerinRange 0 (- (Utilities|Array|Length _available_meshes) 1)))))

(event Collision|EventActorBeginOverlap
  (params (OtherActor :type Actor%20Object%20Reference)))

(event EventTick
  (params (DeltaSeconds :type Float%20%28single-precision%29)))

(event EventBeginPlay
  ;[1 1 1] Random Mesh
  (bind _aswilliams_player_bp (Utilities|Casting|CastToWilliams_Player_BP (Game|GetPlayerCharacter 0)))
  (Variables|Default|SetAs%20Williams%20Player%20BP _aswilliams_player_bp)
  (CallFunction|SetRandomMesh)
  (bind _aspick_up_wb (Utilities|Casting|CastToPickUp_WB (UserInterface|GetWidget (Variables|Default|GetE_PickUp_Widget))))
  (bind _output_get (Variables|Default|SetWidget0 _aspick_up_wb))
  (Default|ChangeItemName _output_get (Utilities|Text|ToText(String) (Variables|Default|GetName)))
  (Default|ShowEatText _output_get))

(event EventPickUp
  (bind _as_williams_player_bp (Variables|Default|GetAs%20Williams%20Player%20BP))
  (bind _item (Variables|Default|GetItem))
  (bind _returnvalue (Transformation|GetWorldLocation _item))
  (bind _rootcomponent (Variables|/Script/Engine.Actor|GetRootComponent _as_williams_player_bp))
  (bind _returnvalue_2 (Transformation|GetWorldLocation _rootcomponent))
  (Widget|SetVisibility (Variables|Default|GetWidget0) "Hidden")
  (bind _aswilliams_player_bp (Utilities|Casting|CastToWilliams_Player_BP (Game|GetPlayerCharacter 0)))
  (Variables|/Game/Williams_E/Blueprints/Player/Williams_Player_BP.Williams_Player_BP_C|SetFood _aswilliams_player_bp (+ (Variables|/Game/Williams_E/Blueprints/Player/Williams_Player_BP.Williams_Player_BP_C|GetFood _aswilliams_player_bp) 1))
  (bind _itemadded (Default|AddtoInventory (Actor|GetComponentbyClass _aswilliams_player_bp "/Game/Sean_H/Inventory/Comp_Inventory.Comp_Inventory_C") (Variables|Default|GetInventory_0)))
  (if _itemadded
    (bind _foundwidgets (Widget|GetAllWidgetsOfClass "/Game/Sean_H/Inventory/W_Inventory.W_Inventory_C" true))
    ;[0.1596 0.6662 1] Pickup Sound (Luis)
    (Audio|PlaySound2D "/Game/Robles_Delgado_L/Sounds/Player-Sounds/Item/Robles_Item_Pickup.Robles_Item_Pickup" 1.0 1.0 0.0 0 0)
    (Utilities|IsValid (Utilities|Array|Get(acopy) _foundwidgets)
      (:Is%20Valid
        (Default|SetGrid (Utilities|Array|Get(acopy) _foundwidgets)))
      (:Is%20Not%20Valid
        _))
    (Collision|SetCollisionEnabled (Variables|Default|GetItem) "NoCollision")
    (bind _pickup (Timeline|Timeline Play)
      (:Update
        (Transformation|SetWorldLocation _item (Math|Vector|MakeVector (Math|Float|Lerp (.x _returnvalue) (.x _returnvalue_2) _pickup) (Math|Float|Lerp (.y _returnvalue) (.y _returnvalue_2) _pickup) (Math|Float|Lerp (.z _returnvalue) (- (.z _returnvalue_2) 3e+01) _pickup)) false false))
      (:Finished
        (Actor|DestroyActor)))))

(fn ConstructionScript)

(fn Eat
  (Development|PrintString "Ate")
  ;[1 1 1] For Luis
  (Audio|PlaySound2D "/Game/Robles_Delgado_L/Sounds/Player-Sounds/Item/Robles_Food_Eat.Robles_Food_Eat" 1.0 1.0 0.0 0 0)
  (CallFunction|DestroyFood)
  (return (Variables|Default|GetHungerAmount)))
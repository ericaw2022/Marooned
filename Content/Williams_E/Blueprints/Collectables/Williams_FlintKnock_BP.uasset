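; Flintknock gun pickup that the player collects through an Interact event.
; On interact it sets HasFlintknock on Williams_Player_BP and tries to add its Inventory item to the player's Comp_Inventory.
; On success it plays a pickup sound, refreshes the W_Inventory grid and destroys itself, otherwise it prints that the inventory is full.
; The HasFlintknock flag is set before the inventory check, so it stays true even when the add fails.
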(event EventInteract
  (bind _aswilliams_player_bp (Utilities|Casting|CastToWilliams_Player_BP (Game|GetPlayerCharacter 0)))
  (Variables|/Game/Williams_E/Blueprints/Player/Williams_Player_BP.Williams_Player_BP_C|SetHasFlintknock? _aswilliams_player_bp true)
  (bind _itemadded (Default|AddtoInventory (Actor|GetComponentbyClass _aswilliams_player_bp "/Game/Sean_H/Inventory/Comp_Inventory.Comp_Inventory_C") (Variables|Default|GetInventory)))
  (if _itemadded
    (bind _foundwidgets (Widget|GetAllWidgetsOfClass "/Game/Sean_H/Inventory/W_Inventory.W_Inventory_C" true))
    ;[0.1596 0.6662 1] Pickup Sound (Luis)
    (Audio|PlaySound2D "/Game/Robles_Delgado_L/Sounds/Player-Sounds/Item/Robles_Item_Pickup.Robles_Item_Pickup" 1.0 1.0 0.0 0 0)
    (Utilities|IsValid (Utilities|Array|Get(acopy) _foundwidgets)
      (:Is%20Valid
        (Default|SetGrid (Utilities|Array|Get(acopy) _foundwidgets)))
      (:Is%20Not%20Valid
        _))
    (Actor|DestroyActor)
    (Development|PrintString "Gun collected!")
    (else
      (Development|PrintString "Inventory Full"))))

(fn ConstructionScript)
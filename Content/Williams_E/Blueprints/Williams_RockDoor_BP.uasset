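; Williams_RockDoor_BP is a two-piece rock door that opens a cave once the player has the key.
; PickUpKey sets a HasKey flag, and Interact does nothing until that flag is set.
; A timeline then lerps the left and right rocks' relative X between start and end values, calling the Spawner's CaveUnlockedMessage on every update tick.
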(event EventInteract
  (if (Variables|Default|GetHasKey?)
    (bind _doortrack (Timeline|DoorTimeline Play)
      (:Update
        (Transformation|SetRelativeLocation (Variables|Default|GetRockLeft) (Math|Vector|MakeVector (Math|Float|Lerp (Variables|Default|GetLeftDoorStart) (Variables|Default|GetLeftDoorEnd) _doortrack) 0.0 0.0) false false)
        (Transformation|SetRelativeLocation (Variables|Default|GetRockRight) (Math|Vector|MakeVector (Math|Float|Lerp (Variables|Default|GetRightDoorStart) (Variables|Default|GetRightDoorEnd) _doortrack) 0.0 0.0) false false)
        (Class|WilliamsEnemySpawnBPI|CaveUnlocked(Message) (Variables|Default|GetSpawner))))))

(event EventPickUpKey
  (Variables|Default|SetHasKey? true))

(fn ConstructionScript)
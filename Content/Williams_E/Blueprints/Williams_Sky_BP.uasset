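; Sky actor Blueprint that drives a day-night cycle by rotating a sun and a moon directional light.
; Each Tick advances a 24-hour Time value by delta seconds divided by TimeDialation, resetting it to zero at 24.
; Time maps to a full 360-degree pitch rotation, with the moon light offset 180 degrees from the sun.
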(event EventBeginPlay)

(event Collision|EventActorBeginOverlap
  (params (OtherActor :type Actor%20Object%20Reference)))

(event EventTick
  (params (DeltaSeconds :type Float%20%28single-precision%29))
  (bind _output_get (Variables|Default|SetTime (+ (/ DeltaSeconds (Variables|Default|GetTimeDialation)) (Variables|Default|GetTime))))
  (if (>= _output_get 24.0)
    (Variables|Default|SetTime 0.0)
    (else
      (Transformation|SetRelativeRotation (Variables|Default|GetDirectionalLight) (Math|Rotator|MakeRotator 0.0 (* (/ (Variables|Default|GetTime) 24.0) 3.6e+02) 0.0) false false)
      (Transformation|SetRelativeRotation (Variables|Default|GetDirectionalLight_Moon) (Math|Rotator|MakeRotator 0.0 (+ (* (/ (Variables|Default|GetTime) 24.0) 3.6e+02) 1.8e+02) 0.0) false false))))

(fn ConstructionScript)
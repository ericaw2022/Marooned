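; Enemy spawner Blueprint that creates groups of Williams_Enemy_Base_BP enemies around its location.
; SpawnEnemy picks a random group size, places each enemy at a random reachable navmesh point within a radius, increments a count and prints a debug message.
; A looping random-interval timer gated by a maximum enemy count is built but disconnected, and CaveUnlocked is empty, so nothing here triggers spawning.
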(event Custom|Spawn%20Enemy
  (for _index (range 0 (Math|Random|RandomIntegerinRange (Variables|Default|GetMinEnemiesInGroup) (Variables|Default|GetMaxEnemiesInGroup)))
    (Game|SpawnActorfromClass "/Game/Williams_E/Blueprints/Enemies/Williams_Enemy_Base_BP.Williams_Enemy_Base_BP_C" (Math|Transform|MakeTransform (.RandomLocation (AI|Navigation|GetRandomReachablePointinRadius (Transformation|GetActorLocation) (Variables|Default|GetEnemySpawnAreaRadius) 0 0)) "0, 0, 0" "1.000000,1.000000,1.000000") "AdjustIfPossibleButAlwaysSpawn" "MultiplyWithRoot" 0 0)
    (Variables|Default|SetCurrentEnemyCount (+ (Variables|Default|GetCurrentEnemyCount) 1.0))
    (Development|PrintString "Enemy Spawned")))

(event EventCaveUnlocked)

(fn ConstructionScript)
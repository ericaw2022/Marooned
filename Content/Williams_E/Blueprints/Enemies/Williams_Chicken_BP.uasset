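; Chicken AI pawn with a random mesh that can be killed for meat and flags player sightings on its Blackboard via PawnSensing.
; Damage plays hit sounds based on the player's equipped weapon and reduces health.
; At zero health, a timeline tips the mesh over with a poof effect, then destroys it, spawns a meat actor and notifies the chicken spawner.
; A separate SpawnAnim event scales the mesh in and marks it alive.
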(event OnSeePawn(PawnSensing)
  (params (Pawn :type Pawn%20Object%20Reference))
  ;[1 1 1] Sees player
  (Utilities|Casting|CastToWilliams_Player_BP Pawn)
  (AI|Components|Blackboard|SetValueasBool (AI|GetBlackboard (AI|GetAIController self)) (Utilities|Name|MakeLiteralName "HasSeenPlayer?") true))

(event Custom|SetRandomMesh
  (bind _availablemeshes (Variables|Default|GetAvailableMeshes))
  ;[1 1 1] Random skeletal mesh spawning
  (Components|SkeletalMesh|SetSkeletalMeshAsset (Variables|Character|GetMesh) (Utilities|Array|Get(acopy) _availablemeshes (Math|Random|RandomIntegerinRange 0 (- (Utilities|Array|Length _availablemeshes) 1)))))

(event Custom|SpawnAnim
  (bind _spawn (Timeline|Timeline Play)
    (:Update
      (Transformation|SetWorldScale3D (Variables|Character|GetMesh) (Math|Conversions|ToVector(Float) (Math|Float|Lerp 0.0 1.0 _spawn)))
      (Variables|Default|SetIsChickenAlive? true))))

(event Custom|DeathSequence
  (bind _spawn (Timeline|Timeline_0 Play)
    (:Update
      (Transformation|SetRelativeRotation (Variables|Character|GetMesh) (Math|Rotator|MakeRotator 0.0 (Math|Float|Lerp 0.0 9e+01 _spawn) 0.0) false false)
      (Components|Activation|Activate (Variables|Default|GetDeathPoof) false))
    (:Finished
      (Actor|DestroyActor)
      (bind _returnvalue (Game|SpawnActorfromClass :Class "/Game/Williams_E/Blueprints/Collectables/Williams_ChickenMeat_BP.Williams_ChickenMeat_BP_C" :SpawnTransform (Math|Conversions|ToTransform(Vector) (Transformation|GetActorLocation)) :CollisionHandlingOverride "Undefined" :TransformScaleMethod "MultiplyWithRoot" :Image 0 :Crafting%20Item 0 :Instigator 0))
      (Default|StopPhysics _returnvalue)
      (bind _returnvalue_2 (Actor|GetActorOfClass "/Game/Williams_E/Blueprints/Enemies/Williams_Chicken_Spawner_BP.Williams_Chicken_Spawner_BP_C"))
      (Default|EnemyKilled _returnvalue_2))))

(event Collision|EventActorBeginOverlap
  (params (OtherActor :type Actor%20Object%20Reference)))

(event EventBeginPlay
  ;[1 1 1] Random skeletal mesh spawning
  (CallFunction|SetRandomMesh))

(event Game|Damage|EventAnyDamage
  (params (Damage :type Float%20%28single-precision%29) (DamageType :type Damage%20Type%20Object%20Reference) (InstigatedBy :type Controller%20Object%20Reference) (DamageCauser :type Actor%20Object%20Reference))
  ;[1 1 1] Damage received by ai
  ;;[0.000291 0.5565 1] Weapon hit sounds
  (bind _outactors (Actor|GetAllActorsOfClass "/Game/Williams_E/Blueprints/Player/Williams_Player_BP.Williams_Player_BP_C"))
  (Utilities|FlowControl|Sequence
    (:then_0
      (if (Variables|/Game/Williams_E/Blueprints/Player/Williams_Player_BP.Williams_Player_BP_C|GetIsGunEquipped? (Utilities|Array|Get(acopy) _outactors))
        (Audio|PlaySound2D "/Game/Robles_Delgado_L/Sounds/Player-Sounds/Flintlock/Robles_FlintlockHit.Robles_FlintlockHit" 1.0 1.0 0.0 0 0)
        ;;[0.02034 0.4278 1] Damage Sound
        (Audio|PlaySoundatLocation "/Game/Robles_Delgado_L/Sounds/AI-Sounds/Chicken/Robles_Chicken_Hit.Robles_Chicken_Hit" (Transformation|GetActorLocation) "0, 0, 0" 1.0 1.0 0.0 0 0 0 0 :!label _label)
        (Variables|Default|SetHealth (- (Variables|Default|GetHealth) Damage))
        (if (<= (Variables|Default|GetHealth) 0.0)
          (Variables|Default|SetIsChickenAlive? false)
          (CallFunction|DeathSequence))))
    (:then_1
      (if (Variables|/Game/Williams_E/Blueprints/Player/Williams_Player_BP.Williams_Player_BP_C|GetIsSwordEquiped? (Utilities|Array|Get(acopy) _outactors))
        (Audio|PlaySound2D "/Game/Robles_Delgado_L/Sounds/Player-Sounds/Sword/Robles_SwordHit.Robles_SwordHit" 1.0 1.0 0.0 0 0)
        (goto _label)))
    (:then_2
      (if (Variables|/Game/Williams_E/Blueprints/Player/Williams_Player_BP.Williams_Player_BP_C|GetIsPunchEquiped? (Utilities|Array|Get(acopy) _outactors))
        (Audio|PlaySound2D "/Game/Robles_Delgado_L/Sounds/Robles_AI_Punch.Robles_AI_Punch" 1.0 1.0 0.0 0 0)
        (goto _label)))))

(fn ConstructionScript)
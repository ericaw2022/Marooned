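; Raft construction sign that tracks the player's resources and builds the raft in six sequential stages, from base to skull keepsake.
; Tick refreshes the paper widget's have/required counters and runs Logic, a nested check that latches each stage's CanBuild flag.
; Player overlap builds the next affordable stage on Williams_Raft_BP, deducts its cost, and switches widget pages for completed stages.
; Having the cave key switches the widget to page 1.
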(event OnComponentBeginOverlap(Box)
  (params (OverlappedComponent :type Primitive%20Component%20Object%20Reference) (OtherActor :type Actor%20Object%20Reference) (OtherComp :type Primitive%20Component%20Object%20Reference) (OtherBodyIndex :type Integer) (bFromSweep :type Boolean) (SweepResult :type Hit%20Result%20Structure%20%28by%20ref%29))
  (if (== OtherActor (Game|GetPlayerCharacter 0))
    (if (Variables|CanBuild?|GetCanbuildBase?)
      (if (Variables|IsBuilt?|GetIsBaseBuilt?)
        (Class|WidgetSwitcher|SetActiveWidgetIndex (Variables|/Game/Williams_E/Widgets/Williams_Sign_WB.Williams_Sign_WB_C|GetWidgetSwitcher_338 (Variables|Default|GetWidget)) 2)
        (if (Variables|CanBuild?|GetCanBuildSail?)
          (if (Variables|IsBuilt?|GetIsSailBuilt?)
            (Class|WidgetSwitcher|SetActiveWidgetIndex (Variables|/Game/Williams_E/Widgets/Williams_Sign_WB.Williams_Sign_WB_C|GetWidgetSwitcher_338 (Variables|Default|GetWidget)) 3)
            (if (Variables|CanBuild?|GetCanBuildRudder?)
              (if (Variables|IsBuilt?|GetIsRudderBuilt?)
                (Class|WidgetSwitcher|SetActiveWidgetIndex (Variables|/Game/Williams_E/Widgets/Williams_Sign_WB.Williams_Sign_WB_C|GetWidgetSwitcher_338 (Variables|Default|GetWidget)) 4)
                (if (Variables|CanBuild?|GetCanBuildBed?)
                  (if (Variables|IsBuilt?|GetIsBedBuilt?)
                    (Class|WidgetSwitcher|SetActiveWidgetIndex (Variables|/Game/Williams_E/Widgets/Williams_Sign_WB.Williams_Sign_WB_C|GetWidgetSwitcher_338 (Variables|Default|GetWidget)) 5)
                    (if (Variables|CanBuild?|GetCanBuildFoodCrate?)
                      (if (Variables|IsBuilt?|GetIsFoodCrateBuilt?)
                        (Class|WidgetSwitcher|SetActiveWidgetIndex (Variables|/Game/Williams_E/Widgets/Williams_Sign_WB.Williams_Sign_WB_C|GetWidgetSwitcher_338 (Variables|Default|GetWidget)) 6)
                        (if (Variables|CanBuild?|GetCanBuildSkull?)
                          (CallFunction|BuildSkull)
                          (Class|WidgetSwitcher|SetActiveWidgetIndex (Variables|/Game/Williams_E/Widgets/Williams_Sign_WB.Williams_Sign_WB_C|GetWidgetSwitcher_338 (Variables|Default|GetWidget)) 7))
                        (else
                          (CallFunction|BuildCrate))))
                    (else
                      (CallFunction|BuildBed))))
                (else
                  (CallFunction|BuildRudder))))
            (else
              (CallFunction|BuildSail))))
        (else
          (CallFunction|BuildBase))))))

(event Custom|GotCaveKey
  (bind _aswilliams_player_bp (Utilities|Casting|CastToWilliams_Player_BP (Game|GetPlayerCharacter 0)))
  (Variables|Default|SetMyPlayer _aswilliams_player_bp)
  (bind _aswilliams_sign_wb (Utilities|Casting|CastToWilliams_Sign_WB (UserInterface|GetWidget (Variables|Default|GetPaperWidget))))
  (Variables|Default|SetWidget _aswilliams_sign_wb)
  (if (Variables|/Game/Williams_E/Blueprints/Player/Williams_Player_BP.Williams_Player_BP_C|GetHasCaveKey? (Variables|Default|GetMyPlayer))
    (Class|WidgetSwitcher|SetActiveWidgetIndex (Variables|/Game/Williams_E/Widgets/Williams_Sign_WB.Williams_Sign_WB_C|GetWidgetSwitcher_338 (Variables|Default|GetWidget)) 1)))

(event Custom|BuildBase
  (bind _myplayer (Variables|Default|GetMyPlayer))
  (bind _myplayer_2 (Variables|Default|GetMyPlayer))
  (bind _returnvalue (Actor|GetActorOfClass "/Game/Williams_E/Blueprints/Williams_Raft_BP.Williams_Raft_BP_C"))
  (Default|BuildBase _returnvalue)
  (Variables|/Game/Williams_E/Blueprints/Player/Williams_Player_BP.Williams_Player_BP_C|SetBranches _myplayer_2 (- (Variables|/Game/Williams_E/Blueprints/Player/Williams_Player_BP.Williams_Player_BP_C|GetBranches _myplayer) (Variables|RequiredItems|GetRequiredBranchesForBase)))
  (Variables|/Game/Williams_E/Blueprints/Player/Williams_Player_BP.Williams_Player_BP_C|SetWoodPlanks _myplayer_2 (- (Variables|/Game/Williams_E/Blueprints/Player/Williams_Player_BP.Williams_Player_BP_C|GetWoodPlanks _myplayer) (Variables|RequiredItems|GetRequiredWoodPlanksForBase)))
  (Variables|/Game/Williams_E/Blueprints/Player/Williams_Player_BP.Williams_Player_BP_C|SetTwine _myplayer_2 (- (Variables|/Game/Williams_E/Blueprints/Player/Williams_Player_BP.Williams_Player_BP_C|GetTwine _myplayer) (Variables|RequiredItems|GetRequiredTwineForBase)))
  (Variables|IsBuilt?|SetIsBaseBuilt? true))

(event Custom|Build%20sail
  (bind _myplayer (Variables|Default|GetMyPlayer))
  (bind _myplayer_2 (Variables|Default|GetMyPlayer))
  (bind _returnvalue (Actor|GetActorOfClass "/Game/Williams_E/Blueprints/Williams_Raft_BP.Williams_Raft_BP_C"))
  (Default|BuildSail _returnvalue)
  (Variables|/Game/Williams_E/Blueprints/Player/Williams_Player_BP.Williams_Player_BP_C|SetTwine _myplayer_2 (- (Variables|/Game/Williams_E/Blueprints/Player/Williams_Player_BP.Williams_Player_BP_C|GetTwine _myplayer) (Variables|RequiredItems|GetRequiredTwineForMast)))
  (Variables|/Game/Williams_E/Blueprints/Player/Williams_Player_BP.Williams_Player_BP_C|SetBones _myplayer_2 (- (Variables|/Game/Williams_E/Blueprints/Player/Williams_Player_BP.Williams_Player_BP_C|GetBones _myplayer) (Variables|RequiredItems|GetRequiredBonesForMast)))
  (Variables|/Game/Williams_E/Blueprints/Player/Williams_Player_BP.Williams_Player_BP_C|SetBranches _myplayer_2 (- (Variables|/Game/Williams_E/Blueprints/Player/Williams_Player_BP.Williams_Player_BP_C|GetBranches _myplayer) (Variables|RequiredItems|GetRequiredBranchesForMast)))
  (Variables|/Game/Williams_E/Blueprints/Player/Williams_Player_BP.Williams_Player_BP_C|SetSail _myplayer_2 (- (Variables|/Game/Williams_E/Blueprints/Player/Williams_Player_BP.Williams_Player_BP_C|GetSail _myplayer) (Variables|RequiredItems|GetRequiredSail)))
  (Variables|IsBuilt?|SetIsSailBuilt? true))

(event Custom|Build%20Rudder
  (bind _myplayer (Variables|Default|GetMyPlayer))
  (bind _returnvalue (Actor|GetActorOfClass "/Game/Williams_E/Blueprints/Williams_Raft_BP.Williams_Raft_BP_C"))
  (Default|BuildRudder _returnvalue)
  (Variables|/Game/Williams_E/Blueprints/Player/Williams_Player_BP.Williams_Player_BP_C|SetWoodPlanks _myplayer (- (Variables|/Game/Williams_E/Blueprints/Player/Williams_Player_BP.Williams_Player_BP_C|GetWoodPlanks _myplayer) (Variables|RequiredItems|GetRequiredPlanksForRudder)))
  (Variables|IsBuilt?|SetIsRudderBuilt? true))

(event Custom|Build%20Bed
  (bind _myplayer (Variables|Default|GetMyPlayer))
  (bind _myplayer_2 (Variables|Default|GetMyPlayer))
  (bind _returnvalue (Actor|GetActorOfClass "/Game/Williams_E/Blueprints/Williams_Raft_BP.Williams_Raft_BP_C"))
  (Default|BuildBed _returnvalue)
  (Variables|/Game/Williams_E/Blueprints/Player/Williams_Player_BP.Williams_Player_BP_C|SetPalmLeaves _myplayer_2 (- (Variables|/Game/Williams_E/Blueprints/Player/Williams_Player_BP.Williams_Player_BP_C|GetPalmLeaves _myplayer) (Variables|RequiredItems|GetRequiredLeavesForBed)))
  (Variables|/Game/Williams_E/Blueprints/Player/Williams_Player_BP.Williams_Player_BP_C|SetStones _myplayer_2 (- (Variables|/Game/Williams_E/Blueprints/Player/Williams_Player_BP.Williams_Player_BP_C|GetStones _myplayer) (Variables|RequiredItems|GetRequiredStonesForBed)))
  (Variables|IsBuilt?|SetIsBedBuilt? true))

(event Custom|Build%20Crate
  (bind _myplayer (Variables|Default|GetMyPlayer))
  (bind _myplayer_2 (Variables|Default|GetMyPlayer))
  (bind _returnvalue (Actor|GetActorOfClass "/Game/Williams_E/Blueprints/Williams_Raft_BP.Williams_Raft_BP_C"))
  (Default|BuildCrate _returnvalue)
  (Variables|/Game/Williams_E/Blueprints/Player/Williams_Player_BP.Williams_Player_BP_C|SetFood _myplayer (- (Variables|/Game/Williams_E/Blueprints/Player/Williams_Player_BP.Williams_Player_BP_C|GetFood _myplayer_2) (Variables|RequiredItems|GetRequiredFoodForCrate)))
  (Variables|/Game/Williams_E/Blueprints/Player/Williams_Player_BP.Williams_Player_BP_C|SetWoodPlanks _myplayer (- (Variables|/Game/Williams_E/Blueprints/Player/Williams_Player_BP.Williams_Player_BP_C|GetWoodPlanks _myplayer_2) (Variables|RequiredItems|GetRequiredPlanksForCrate)))
  (Variables|IsBuilt?|SetIsFoodCrateBuilt? true))

(event Custom|Build%20Skull
  (bind _myplayer (Variables|Default|GetMyPlayer))
  (bind _returnvalue (Actor|GetActorOfClass "/Game/Williams_E/Blueprints/Williams_Raft_BP.Williams_Raft_BP_C"))
  (Default|BuildSkull _returnvalue)
  (Variables|/Game/Williams_E/Blueprints/Player/Williams_Player_BP.Williams_Player_BP_C|SetBones _myplayer (- (Variables|/Game/Williams_E/Blueprints/Player/Williams_Player_BP.Williams_Player_BP_C|GetBones _myplayer) (Variables|RequiredItems|GetRequiredBonesNeededForSkull)))
  (Variables|Default|SetIsRaftComplete? true))

(event Custom|Logic
  (bind _myplayer (Variables|Default|GetMyPlayer))
  (bind _myplayer_2 (Variables|Default|GetMyPlayer))
  (bind _myplayer_3 (Variables|Default|GetMyPlayer))
  (bind _myplayer_4 (Variables|Default|GetMyPlayer))
  (if (Math|Boolean|ANDBoolean (>= (Variables|/Game/Williams_E/Blueprints/Player/Williams_Player_BP.Williams_Player_BP_C|GetTwine _myplayer_2) (Variables|RequiredItems|GetRequiredTwineForBase)) (>= (Variables|/Game/Williams_E/Blueprints/Player/Williams_Player_BP.Williams_Player_BP_C|GetWoodPlanks _myplayer_2) (Variables|RequiredItems|GetRequiredWoodPlanksForBase)) (>= (Variables|/Game/Williams_E/Blueprints/Player/Williams_Player_BP.Williams_Player_BP_C|GetBranches _myplayer_2) (Variables|RequiredItems|GetRequiredBranchesForBase)))
    (Variables|CanBuild?|SetCanbuildBase? true)
    (if (Variables|IsBuilt?|GetIsBaseBuilt?)
      (if (Math|Boolean|ANDBoolean (>= (Variables|/Game/Williams_E/Blueprints/Player/Williams_Player_BP.Williams_Player_BP_C|GetTwine _myplayer) (Variables|RequiredItems|GetRequiredTwineForMast)) (>= (Variables|/Game/Williams_E/Blueprints/Player/Williams_Player_BP.Williams_Player_BP_C|GetBones _myplayer) (Variables|RequiredItems|GetRequiredBonesForMast)) (>= (Variables|/Game/Williams_E/Blueprints/Player/Williams_Player_BP.Williams_Player_BP_C|GetBranches _myplayer) (Variables|RequiredItems|GetRequiredBranchesForMast)) (>= (Variables|/Game/Williams_E/Blueprints/Player/Williams_Player_BP.Williams_Player_BP_C|GetSail _myplayer) (Variables|RequiredItems|GetRequiredSail)))
        (Variables|CanBuild?|SetCanBuildSail? true)
        (if (Variables|IsBuilt?|GetIsSailBuilt?)
          (if (>= (Variables|/Game/Williams_E/Blueprints/Player/Williams_Player_BP.Williams_Player_BP_C|GetWoodPlanks (Variables|Default|GetMyPlayer)) (Variables|RequiredItems|GetRequiredPlanksForRudder))
            (Variables|CanBuild?|SetCanBuildRudder? true)
            (if (Variables|IsBuilt?|GetIsRudderBuilt?)
              (if (and (>= (Variables|/Game/Williams_E/Blueprints/Player/Williams_Player_BP.Williams_Player_BP_C|GetPalmLeaves _myplayer_3) (Variables|RequiredItems|GetRequiredLeavesForBed)) (>= (Variables|/Game/Williams_E/Blueprints/Player/Williams_Player_BP.Williams_Player_BP_C|GetStones _myplayer_3) (Variables|RequiredItems|GetRequiredStonesForBed)))
                (Variables|CanBuild?|SetCanBuildBed? true)
                (if (Variables|IsBuilt?|GetIsBedBuilt?)
                  (if (and (>= (Variables|/Game/Williams_E/Blueprints/Player/Williams_Player_BP.Williams_Player_BP_C|GetFood _myplayer_4) (Variables|RequiredItems|GetRequiredFoodForCrate)) (>= (Variables|/Game/Williams_E/Blueprints/Player/Williams_Player_BP.Williams_Player_BP_C|GetWoodPlanks _myplayer_4) (Variables|RequiredItems|GetRequiredPlanksForCrate)))
                    (Variables|CanBuild?|SetCanBuildFoodCrate? true)
                    (if (Variables|IsBuilt?|GetIsFoodCrateBuilt?)
                      (if (>= (Variables|/Game/Williams_E/Blueprints/Player/Williams_Player_BP.Williams_Player_BP_C|GetBones (Variables|Default|GetMyPlayer)) (Variables|RequiredItems|GetRequiredBonesNeededForSkull))
                        (Variables|CanBuild?|SetCanBuildSkull? true)))))))))))))

(event EventBeginPlay
  (bind _aswilliams_player_bp (Utilities|Casting|CastToWilliams_Player_BP (Game|GetPlayerCharacter 0)))
  (Variables|Default|SetMyPlayer _aswilliams_player_bp)
  (bind _aswilliams_sign_wb (Utilities|Casting|CastToWilliams_Sign_WB (UserInterface|GetWidget (Variables|Default|GetPaperWidget))))
  (Variables|Default|SetWidget _aswilliams_sign_wb)
  (if (Variables|/Game/Williams_E/Blueprints/Player/Williams_Player_BP.Williams_Player_BP_C|GetHasCaveKey? (Variables|Default|GetMyPlayer))
    (Class|WidgetSwitcher|SetActiveWidgetIndex (Variables|/Game/Williams_E/Widgets/Williams_Sign_WB.Williams_Sign_WB_C|GetWidgetSwitcher_338 (Variables|Default|GetWidget)) 1)))

(event EventTick
  (params (DeltaSeconds :type Float%20%28single-precision%29))
  (bind _widget (Variables|Default|GetWidget))
  (bind _myplayer (Variables|Default|GetMyPlayer))
  (bind _myplayer_2 (Variables|Default|GetMyPlayer))
  (bind _myplayer_3 (Variables|Default|GetMyPlayer))
  (bind _widget_2 (Variables|Default|GetWidget))
  (bind _myplayer_4 (Variables|Default|GetMyPlayer))
  (bind _widget_3 (Variables|Default|GetWidget))
  (bind _widget_4 (Variables|Default|GetWidget))
  (Rendering|Components|TextRender|SetText (Variables|/Game/Williams_E/Widgets/Williams_Sign_WB.Williams_Sign_WB_C|GetBranchesNeeded _widget_2) (Utilities|Text|ToText(String) (Utilities|String|Append (Utilities|String|ToString(Integer) (Variables|/Game/Williams_E/Blueprints/Player/Williams_Player_BP.Williams_Player_BP_C|GetBranches _myplayer_4)) "/" (Utilities|String|ToString(Integer) (Variables|RequiredItems|GetRequiredBranchesForBase)))))
  (Rendering|Components|TextRender|SetText (Variables|/Game/Williams_E/Widgets/Williams_Sign_WB.Williams_Sign_WB_C|GetPlanksNeeded _widget_2) (Utilities|Text|ToText(String) (Utilities|String|Append (Utilities|String|ToString(Integer) (Variables|/Game/Williams_E/Blueprints/Player/Williams_Player_BP.Williams_Player_BP_C|GetWoodPlanks _myplayer_4)) "/" (Utilities|String|ToString(Integer) (Variables|RequiredItems|GetRequiredWoodPlanksForBase)))))
  (Rendering|Components|TextRender|SetText (Variables|/Game/Williams_E/Widgets/Williams_Sign_WB.Williams_Sign_WB_C|GetTwineNeeded _widget_2) (Utilities|Text|ToText(String) (Utilities|String|Append (Utilities|String|ToString(Integer) (Variables|/Game/Williams_E/Blueprints/Player/Williams_Player_BP.Williams_Player_BP_C|GetTwine _myplayer_4)) "/" (Utilities|String|ToString(Integer) (Variables|RequiredItems|GetRequiredTwineForBase)))))
  (Rendering|Components|TextRender|SetText (Variables|/Game/Williams_E/Widgets/Williams_Sign_WB.Williams_Sign_WB_C|GetTwineNeededForMast _widget_3) (Utilities|Text|ToText(String) (Utilities|String|Append (Utilities|String|ToString(Integer) (Variables|/Game/Williams_E/Blueprints/Player/Williams_Player_BP.Williams_Player_BP_C|GetTwine _myplayer)) "/" (Utilities|String|ToString(Integer) (Variables|RequiredItems|GetRequiredTwineForMast)))))
  (Rendering|Components|TextRender|SetText (Variables|/Game/Williams_E/Widgets/Williams_Sign_WB.Williams_Sign_WB_C|GetBonesNeededForMast _widget_3) (Utilities|Text|ToText(String) (Utilities|String|Append (Utilities|String|ToString(Integer) (Variables|/Game/Williams_E/Blueprints/Player/Williams_Player_BP.Williams_Player_BP_C|GetBones _myplayer)) "/" (Utilities|String|ToString(Integer) (Variables|RequiredItems|GetRequiredBonesForMast)))))
  (Rendering|Components|TextRender|SetText (Variables|/Game/Williams_E/Widgets/Williams_Sign_WB.Williams_Sign_WB_C|GetBranchesNeededformast _widget_3) (Utilities|Text|ToText(String) (Utilities|String|Append (Utilities|String|ToString(Integer) (Variables|/Game/Williams_E/Blueprints/Player/Williams_Player_BP.Williams_Player_BP_C|GetBranches _myplayer)) "/" (Utilities|String|ToString(Integer) (Variables|RequiredItems|GetRequiredBranchesForMast)))))
  (Rendering|Components|TextRender|SetText (Variables|/Game/Williams_E/Widgets/Williams_Sign_WB.Williams_Sign_WB_C|GetSailNeeded _widget_3) (Utilities|Text|ToText(String) (Utilities|String|Append (Utilities|String|ToString(Integer) (Variables|/Game/Williams_E/Blueprints/Player/Williams_Player_BP.Williams_Player_BP_C|GetSail _myplayer)) "/" (Utilities|String|ToString(Integer) (Variables|RequiredItems|GetRequiredSail)))))
  (Rendering|Components|TextRender|SetText (Variables|/Game/Williams_E/Widgets/Williams_Sign_WB.Williams_Sign_WB_C|GetPlanksneededforrudder (Variables|Default|GetWidget)) (Utilities|Text|ToText(String) (Utilities|String|Append (Utilities|String|ToString(Integer) (Variables|/Game/Williams_E/Blueprints/Player/Williams_Player_BP.Williams_Player_BP_C|GetWoodPlanks (Variables|Default|GetMyPlayer))) "/" (Utilities|String|ToString(Integer) (Variables|RequiredItems|GetRequiredPlanksForRudder)))))
  (Rendering|Components|TextRender|SetText (Variables|/Game/Williams_E/Widgets/Williams_Sign_WB.Williams_Sign_WB_C|GetLeavesneededforbed _widget_4) (Utilities|Text|ToText(String) (Utilities|String|Append (Utilities|String|ToString(Integer) (Variables|/Game/Williams_E/Blueprints/Player/Williams_Player_BP.Williams_Player_BP_C|GetPalmLeaves _myplayer_2)) "/" (Utilities|String|ToString(Integer) (Variables|RequiredItems|GetRequiredLeavesForBed)))))
  (Rendering|Components|TextRender|SetText (Variables|/Game/Williams_E/Widgets/Williams_Sign_WB.Williams_Sign_WB_C|GetStonesneededforbed _widget_4) (Utilities|Text|ToText(String) (Utilities|String|Append (Utilities|String|ToString(Integer) (Variables|/Game/Williams_E/Blueprints/Player/Williams_Player_BP.Williams_Player_BP_C|GetStones _myplayer_2)) "/" (Utilities|String|ToString(Integer) (Variables|RequiredItems|GetRequiredStonesForBed)))))
  (Rendering|Components|TextRender|SetText (Variables|/Game/Williams_E/Widgets/Williams_Sign_WB.Williams_Sign_WB_C|GetFruitneededforfood _widget) (Utilities|Text|ToText(String) (Utilities|String|Append (Utilities|String|ToString(Integer) (Variables|/Game/Williams_E/Blueprints/Player/Williams_Player_BP.Williams_Player_BP_C|GetFood _myplayer_3)) "/" (Utilities|String|ToString(Integer) (Variables|RequiredItems|GetRequiredFoodForCrate)))))
  (Rendering|Components|TextRender|SetText (Variables|/Game/Williams_E/Widgets/Williams_Sign_WB.Williams_Sign_WB_C|GetPlanksneededforfoodcrate _widget) (Utilities|Text|ToText(String) (Utilities|String|Append (Utilities|String|ToString(Integer) (Variables|/Game/Williams_E/Blueprints/Player/Williams_Player_BP.Williams_Player_BP_C|GetWoodPlanks _myplayer_3)) "/" (Utilities|String|ToString(Integer) (Variables|RequiredItems|GetRequiredPlanksForCrate)))))
  (Rendering|Components|TextRender|SetText (Variables|/Game/Williams_E/Widgets/Williams_Sign_WB.Williams_Sign_WB_C|GetBonesneededforkeepsake (Variables|Default|GetWidget)) (Utilities|Text|ToText(String) (Utilities|String|Append (Utilities|String|ToString(Integer) (Variables|/Game/Williams_E/Blueprints/Player/Williams_Player_BP.Williams_Player_BP_C|GetBones (Variables|Default|GetMyPlayer))) "/" (Utilities|String|ToString(Integer) (Variables|RequiredItems|GetRequiredBonesNeededForSkull)))))
  (CallFunction|Logic))

(fn ConstructionScript)
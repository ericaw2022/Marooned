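; Buildable raft actor that appears piece by piece and triggers the game's ending cutscene once complete.
; All parts start hidden without collision on BeginPlay, and custom Build events reveal them with collision through shared Show/Hide macros.
; Building the skull alone sets RaftComplete, with no check on the other parts.
; When the player overlaps the box with RaftComplete set, the ending Level Sequence plays.
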(event OnComponentBeginOverlap(Box)
  (params (OverlappedComponent :type Primitive%20Component%20Object%20Reference) (OtherActor :type Actor%20Object%20Reference) (OtherComp :type Primitive%20Component%20Object%20Reference) (OtherBodyIndex :type Integer) (bFromSweep :type Boolean) (SweepResult :type Hit%20Result%20Structure%20%28by%20ref%29))
  (if (== OtherActor (Game|GetPlayerCharacter 0))
    ;[1 1 1] Final Cutscene Call on True
    (if (Variables|Default|GetRaftComplete)
      (bind _outactor (Sequencer|Player|CreateLevelSequencePlayer "/Game/Bernabe_N/Sequences/EndingSequence.EndingSequence"))
      (Sequencer|Player|Play (Variables|/Script/LevelSequence.LevelSequenceActor|GetSequencePlayer _outactor) :!class /Script/MovieScene.MovieSceneSequencePlayer))))

(event EventBeginPlay
  (bind _base (Variables|Default|GetBase))
  (bind _rudder (Variables|Default|GetRudder))
  (bind _food (Variables|Default|GetFood))
  (bind _skull (Variables|Default|GetSkull))
  (bind _bed (Variables|Default|GetBed))
  (bind _mast (Variables|Default|GetMast))
  (bind _sail (Variables|Default|GetSail))
  (Utilities|HideMacro _base _base)
  (Utilities|HideMacro _rudder _rudder)
  (Utilities|HideMacro _mast _mast)
  (Utilities|HideMacro _sail _sail)
  (Utilities|HideMacro _food _food)
  (Utilities|HideMacro _skull _skull)
  (Utilities|HideMacro _bed _bed))

(event Collision|EventActorBeginOverlap
  (params (OtherActor :type Actor%20Object%20Reference)))

(event EventTick
  (params (DeltaSeconds :type Float%20%28single-precision%29)))

(event EventBuildBase
  (bind _base (Variables|Default|GetBase))
  (Utilities|ShowMacro _base _base))

(event EventBuildSail
  (bind _mast (Variables|Default|GetMast))
  (bind _sail (Variables|Default|GetSail))
  (Utilities|ShowMacro _mast _mast)
  (Utilities|ShowMacro _sail _sail))

(event EventBuildRudder
  (bind _rudder (Variables|Default|GetRudder))
  (Utilities|ShowMacro _rudder _rudder))

(event EventBuildBed
  (bind _bed (Variables|Default|GetBed))
  (Utilities|ShowMacro _bed _bed))

(event EventBuildCrate
  (bind _food (Variables|Default|GetFood))
  (Utilities|ShowMacro _food _food))

(event EventBuildSkull
  (bind _skull (Variables|Default|GetSkull))
  (Utilities|ShowMacro _skull _skull)
  (Variables|Default|SetRaftComplete true))

(fn ConstructionScript)
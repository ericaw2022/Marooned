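; Interactable journal actor that opens the Journal14 widget when the player interacts with it.
; A sphere overlap with the player character toggles the Journal's custom-depth highlight and shows or hides the PickUp_WB prompt in its InteractWidget component.
; Interact creates the journal widget, adds it to the viewport and switches the player controller to UI-only input with a visible cursor.
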(event OnComponentBeginOverlap(Sphere)
  (params (OverlappedComponent :type Primitive%20Component%20Object%20Reference) (OtherActor :type Actor%20Object%20Reference) (OtherComp :type Primitive%20Component%20Object%20Reference) (OtherBodyIndex :type Integer) (bFromSweep :type Boolean) (SweepResult :type Hit%20Result%20Structure%20%28by%20ref%29))
  (if (== OtherActor (Game|GetPlayerCharacter 0))
    (Rendering|SetRenderCustomDepth (Variables|Default|GetJournal) true)
    (bind _aspick_up_wb (Utilities|Casting|CastToPickUp_WB (UserInterface|GetWidget (Variables|Default|GetInteractWidget))))
    (Widget|SetVisibility _aspick_up_wb "Visible")))

(event OnComponentEndOverlap(Sphere)
  (params (OverlappedComponent :type Primitive%20Component%20Object%20Reference) (OtherActor :type Actor%20Object%20Reference) (OtherComp :type Primitive%20Component%20Object%20Reference) (OtherBodyIndex :type Integer))
  (if (== OtherActor (Game|GetPlayerCharacter 0))
    (Rendering|SetRenderCustomDepth (Variables|Default|GetJournal) false)
    (bind _aspick_up_wb (Utilities|Casting|CastToPickUp_WB (UserInterface|GetWidget (Variables|Default|GetInteractWidget))))
    (Widget|SetVisibility _aspick_up_wb "Hidden")))

(event EventBeginPlay)

(event Collision|EventActorBeginOverlap
  (params (OtherActor :type Actor%20Object%20Reference)))

(event EventTick
  (params (DeltaSeconds :type Float%20%28single-precision%29)))

(event EventInteract
  (bind _returnvalue (Game|GetPlayerController 0))
  ;[1 1 1] Connect this for it to work once you have a widget :)
  (bind _returnvalue_2 (UserInterface|CreateWidget "/Game/Jenkins_Amaris/Widgets/Journals_Pages/Story3/Journal14.Journal14_C"))
  (bind _output_get (Variables|Default|SetNewVar _returnvalue_2))
  (UserInterface|Viewport|AddtoViewport _output_get 0)
  (Input|SetInputModeUIOnly _returnvalue 0 "DoNotLock" false)
  (Variables|/Script/Engine.PlayerController|SetbShowMouseCursor _returnvalue true))

(fn ConstructionScript)
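; Actor component for the crafting system that looks up which items can be crafted at a given craft place.
; GetCraftableItems walks every row of the Williams_CraftableItem_DT data table and returns those whose CraftPlace matches the one passed in.
; On BeginPlay it caches its owner as Character, which the lookup does not use.
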(event EventBeginPlay
  (Variables|Default|SetCharacter (Components|GetOwner)))

(event EventTick
  (params (DeltaSeconds :type Float%20%28single-precision%29)))

(fn GetCraftableItems
  (params (CraftPlace :type Williams_CraftPlace_E%20Enum :default "NewEnumerator0"))
  (bind _outrownames (DataTable|GetDataTableRowNames "/Game/Williams_E/Blueprints/CraftingSystem/Williams_CraftableItem_DT.Williams_CraftableItem_DT"))
  (for _array_element _outrownames
    (bind _returnvalue (Utilities|GetDataTableRow "/Game/Williams_E/Blueprints/CraftingSystem/Williams_CraftableItem_DT.Williams_CraftableItem_DT" _array_element)
      (:then
        (if (Utilities|Enum|Equal(Enum) (.CraftPlace (Utilities|Struct|BreakWilliams_CraftableItem_S _returnvalue)) CraftPlace)
          (Utilities|Array|Add (LocalVariables|GetLocal_Items) _returnvalue)))))
  (return (LocalVariables|GetLocal_Items)))
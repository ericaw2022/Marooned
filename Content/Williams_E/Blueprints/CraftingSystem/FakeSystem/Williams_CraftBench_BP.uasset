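; A crafting bench actor that opens the crafting menu when the player interacts with it.
; When the player enters its box, the bench mesh turns on custom depth and shows a pickup prompt widget, and leaving reverses both and closes the menu.
; Interact creates the crafting widget on first use, then toggles its visibility, switching input mode and mouse cursor and refreshing plank and axe text on opening.
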(event OnComponentBeginOverlap(Box)
  (params (OverlappedComponent :type Primitive%20Component%20Object%20Reference) (OtherActor :type Actor%20Object%20Reference) (OtherComp :type Primitive%20Component%20Object%20Reference) (OtherBodyIndex :type Integer) (bFromSweep :type Boolean) (SweepResult :type Hit%20Result%20Structure%20%28by%20ref%29))
  (if (== OtherActor (Game|GetPlayerCharacter 0))
    (Rendering|SetRenderCustomDepth (Variables|Default|GetBench) true)
    (bind _aspick_up_wb (Utilities|Casting|CastToPickUp_WB (UserInterface|GetWidget (Variables|Default|GetInteractWidget))))
    (Widget|SetVisibility _aspick_up_wb "Visible")))

(event OnComponentEndOverlap(Box)
  (params (OverlappedComponent :type Primitive%20Component%20Object%20Reference) (OtherActor :type Actor%20Object%20Reference) (OtherComp :type Primitive%20Component%20Object%20Reference) (OtherBodyIndex :type Integer))
  (bind _returnvalue (Game|GetPlayerController 0))
  (if (== OtherActor (Game|GetPlayerCharacter 0))
    (Rendering|SetRenderCustomDepth (Variables|Default|GetBench) false)
    (bind _aspick_up_wb (Utilities|Casting|CastToPickUp_WB (UserInterface|GetWidget (Variables|Default|GetInteractWidget))))
    (Widget|SetVisibility _aspick_up_wb "Hidden")
    (Widget|SetVisibility (Variables|Default|GetCraftingMenu) "Hidden")
    (Input|SetInputModeGameOnly _returnvalue false)
    (Variables|/Script/Engine.PlayerController|SetbShowMouseCursor _returnvalue false)))

(event EventInteract
  (bind _returnvalue (Game|GetPlayerController 0))
  (bind _returnvalue_2 (Game|GetPlayerController 0))
  (Utilities|IsValid (Variables|Default|GetCraftingMenu)
    (:Is%20Valid
      (if (Widget|IsVisible (Variables|Default|GetCraftingMenu))
        (Widget|SetVisibility (Variables|Default|GetCraftingMenu) "Hidden")
        (Input|SetInputModeGameOnly _returnvalue false)
        (Variables|/Script/Engine.PlayerController|SetbShowMouseCursor _returnvalue false)
        (else
          (Widget|SetVisibility (Variables|Default|GetCraftingMenu) "Visible")
          (Input|SetInputModeGameandUI _returnvalue_2 0 "DoNotLock" true false :!label _label)
          (Variables|/Script/Engine.PlayerController|SetbShowMouseCursor _returnvalue_2 true)
          (Default|UpdateTextPlank (Variables|Default|GetCraftingMenu))
          (Default|UpdateTextAxe (Variables|Default|GetCraftingMenu)))))
    (:Is%20Not%20Valid
      (bind _returnvalue_3 (UserInterface|CreateWidget "/Game/Williams_E/Blueprints/CraftingSystem/FakeSystem/Williams_Crafting_WB.Williams_Crafting_WB_C"))
      (bind _output_get (Variables|Default|SetCraftingMenu _returnvalue_3))
      (UserInterface|Viewport|AddtoViewport _output_get 0)
      (goto _label))))

(fn ConstructionScript)
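; Crafting component that works out which craftable items from a data table are unlocked at the current level.
; InitCalculateCrafting reads all row names, keeps level-eligible ones in UnlockedCraftableItems and prints them for debugging.
; It requests async loads of unloaded item classes along the way.
; Escape hides the crafting menu and restores game input, but the menu-opening logic is disconnected, and CraftingBenchOpened and PickUpItem are empty stubs.
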(event Custom|CraftingBenchOpened)

(event Custom|InitCalculateCrafting
  (params (Data%20Table%20to%20Use :type Data%20Table%20Object%20Reference))
  (bind _output_get (Variables|Default|SetData%20Table%20To%20Use Data%20Table%20to%20Use))
  (bind _outrownames (DataTable|GetDataTableRowNames _output_get))
  (Variables|Default|SetAllCraftableItems _outrownames)
  (CallFunction|CalculateUnlockedItems)
  (CallFunction|PrintUnlockedItems))

(event Custom|LoadAsync
  (params (NewParam :type A%20Master%20Pick%20Up%20Item%20Soft%20Class%20Reference))
  (Utilities|AsyncLoadClassAsset NewParam))

(event EventBeginPlay)

(event EventTick
  (params (DeltaSeconds :type Float%20%28single-precision%29)))

(event Input|KeyboardEvents|Escape
  (params (Key :type Key%20Structure :default "None"))
  (bind _returnvalue (Game|GetPlayerController 0))
  (:Pressed
    (Widget|SetVisibility (Variables|Default|GetCraftingMenu) "Hidden")
    (Input|SetInputModeGameOnly _returnvalue false)
    (Variables|/Script/Engine.PlayerController|SetbShowMouseCursor _returnvalue false)))

(fn CalculateUnlockedItems
  (for _array_element (Variables|Default|GetAllCraftableItems)
    (LocalVariables|SetCurrentArrayElement _array_element)
    (if (not (Utilities|Array|ContainsItem (Variables|Default|GetUnlockedCraftableItems) (LocalVariables|GetCurrentArrayElement)))
      (bind _out_row (CallFunction|GetCraftableItemfromName (LocalVariables|GetCurrentArrayElement)))
      (LocalVariables|SetCurrentItemRow1 _out_row)
      (if (Utilities|IsValidClass (Utilities|ResolveSoftReference (Utilities|Struct|BreakST_Inventory (LocalVariables|GetCurrentItemRow1))))
        _
        (else
          (CallFunction|LoadAsync (Utilities|Struct|BreakST_Inventory (LocalVariables|GetCurrentItemRow1)))))
      (if (== (Utilities|Struct|BreakST_Inventory (LocalVariables|GetCurrentItemRow1)) 0)
        (Utilities|Array|Add (Variables|Default|GetUnlockedCraftableItems) (LocalVariables|GetCurrentArrayElement) :!label _label)
        (elif (>= (Variables|Default|GetCurrentLvl) (Utilities|Struct|BreakST_Inventory (LocalVariables|GetCurrentItemRow1)))
          (goto _label))))))

(fn GetCraftableItemfromName
  (params (RowName :type Name))
  (bind _returnvalue (Class|DataTableFunctionLibrary|DoesDataTableRowExist (Variables|Default|GetData%20Table%20To%20Use) RowName))
  (if _returnvalue
    (bind _returnvalue_2 (Utilities|GetDataTableRow (Variables|Default|GetData%20Table%20To%20Use) RowName)
      (:then
        (return _returnvalue_2)))))

(fn PrintUnlockedItems
  (for _array_element (Variables|Default|GetUnlockedCraftableItems)
    (Development|PrintString (Utilities|String|ToString(Name) _array_element))))

(fn PickUpItem
  (return ""))
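; Base enemy character Blueprint that spawns with a random skeletal mesh, senses the player and attacks in melee.
; BeginPlay picks a mesh from AvailableMeshes, and seeing the player through PawnSensing sets a "HasSeenPlayer?" Blackboard flag on its AI controller.
; AttackPlayer sphere-traces forward for pawns, plays a punch montage on hitting the player, and damages it if tagged Player.
; Incoming damage reduces Health and destroys the actor at zero.
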(event OnSeePawn(PawnSensing)
  (params (Pawn :type Pawn%20Object%20Reference))
  ;[1 1 1] Sees player
  (Utilities|Casting|CastToWilliams_Player_BP Pawn)
  (AI|Components|Blackboard|SetValueasBool (AI|GetBlackboard (AI|GetAIController self)) (Utilities|Name|MakeLiteralName "HasSeenPlayer?") true))

(event Custom|SetRandomMesh
  (bind _availablemeshes (Variables|Default|GetAvailableMeshes))
  ;[1 1 1] Random skeletal mesh spawning
  (Development|PrintString "Test random mesh")
  (Components|SkeletalMesh|SetSkeletalMeshAsset (Variables|Character|GetMesh) (Utilities|Array|Get(acopy) _availablemeshes (Math|Random|RandomIntegerinRange 0 (- (Utilities|Array|Length _availablemeshes) 1)))))

(event Custom|AttackPlayer
  (bind _returnvalue (Transformation|GetActorLocation))
  ;[1 1 1] Attack player
  (bind (_outhit _returnvalue_2) (Collision|SphereTraceForObjects _returnvalue (+ _returnvalue (* (Math|Vector|GetForwardVector (Transformation|GetActorRotation)) 2.5e+02)) 1.2e+02 (Utilities|Array|MakeArray "ObjectTypeQuery3") false 0 "ForDuration"))
  (if _returnvalue_2
    (Utilities|Casting|CastToWilliams_Player_BP (.HitActor (Collision|BreakHitResult _outhit)))
    (Animation|PlayAnimMontage "/Game/Williams_E/Animations/Fighting/Skeleton_Punch_Montage.Skeleton_Punch_Montage" 1.0 "None")
    (if (Actor|ActorHasTag (.HitActor (Collision|BreakHitResult _outhit)) "Player")
      (Game|Damage|ApplyDamage (.HitActor (Collision|BreakHitResult _outhit)) 1e+01 0 0))))

(event Collision|EventActorBeginOverlap
  (params (OtherActor :type Actor%20Object%20Reference)))

(event EventBeginPlay
  ;[1 1 1] Random skeletal mesh spawning
  (CallFunction|SetRandomMesh))

(event Game|Damage|EventAnyDamage
  (params (Damage :type Float%20%28single-precision%29) (DamageType :type Damage%20Type%20Object%20Reference) (InstigatedBy :type Controller%20Object%20Reference) (DamageCauser :type Actor%20Object%20Reference))
  ;[1 1 1] Damage received by ai
  (Variables|Default|SetHealth (- (Variables|Default|GetHealth) Damage))
  (if (<= (Variables|Default|GetHealth) 0.0)
    (Actor|DestroyActor)
    (else
      (Development|PrintString (Utilities|String|ToString(Float) (Variables|Default|GetHealth))))))

(fn ConstructionScript)